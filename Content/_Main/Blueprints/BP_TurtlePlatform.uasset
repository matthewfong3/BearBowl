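; BP_TurtlePlatform is a turtle that patrols back and forth along X and damages the player character on contact.
; At BeginPlay it derives its endpoints from the sprite's position and the X distance between two widget points.
; A Timeline lerps the actor between them, with a FlipFlop alternating reverse and forward playback and turning it 180 degrees.
; A capsule hit from BP_Character sends that actor a damage message.
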(event `self.ReceiveBeginPlay`
  (bind (_startpos_x _startpos_y _startpos_z) (`KismetMathLibrary.BreakVector` (`self.StartPos`)))
  (bind _startwidget_x (`KismetMathLibrary.BreakVector` (`self.StartWidget`)))
  (bind _endwidget_x (`KismetMathLibrary.BreakVector` (`self.EndWidget`)))
  ; On Begin Play
  (set `self.DeltaX` (`KismetMathLibrary.Abs` (- _startwidget_x _endwidget_x)))
  (set `self.StartPos` (`SceneComponent.K2_GetComponentLocation` (`self.Sprite`)))
  (set `self.EndPos` (`KismetMathLibrary.MakeVector` (+ _startpos_x (`self.DeltaX`)) _startpos_y _startpos_z))
  (`self.Move`))

(event `Move`
  ; Use a Timeline to move the turtle back and forth
  (bind (_direction _alpha) (`Timeline|MovementTimeline` :!via `PlayFromStart` :!label _label)
    (:`Update`
      (`self.K2_SetActorLocation` (`KismetMathLibrary.VLerp` (`self.StartPos`) (`self.EndPos`) _alpha))
      (`self.K2_SetActorRotation` (`KismetMathLibrary.SelectRotator` (`KismetMathLibrary.MakeRotator` 0.0 0.0 0.0) (`KismetMathLibrary.MakeRotator` 0.0 0.0 180.0) (stale _isa))))
    (:`Finished`
      (bind _isa (`/Engine/EditorBlueprintResources/StandardMacros.FlipFlop`)
        (:`A`
          (goto _label :!via `ReverseFromEnd`))
        (:`B`
          (goto _label :!via `PlayFromStart`))))))

(event `self.CapsuleComponent.OnComponentHit`
  (params (HitComponent :type "PrimitiveComponent Object Reference") (OtherActor :type "Actor Object Reference") (OtherComp :type "PrimitiveComponent Object Reference") (NormalImpulse :type "Vector Structure") (Hit :type "HitResult Structure (by ref)"))
  ; When bear collides with turtle
  (if (== (`GameplayStatics.GetObjectClass` OtherActor) "/Game/_Main/Blueprints/BP_Character.BP_Character_C")
    (message `/Game/_Main/Interfaces/BPI_Bear.OnDamage` OtherActor (`self.Damage`))))

(fn `UserConstructionScript`)