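; BP_Flag is a goal flag that ends play when a BP_Character overlaps its Box component.
; The overlap switches on LevelToLoad to show either the WBP_NextLevel widget for one specific value or WBP_WinScreen for any other.
; Both paths then show the mouse cursor, set UI-only input and flag the character as game over.
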(event `self.Box.OnComponentBeginOverlap`
  (params (OverlappedComponent :type "PrimitiveComponent Object Reference") (OtherActor :type "Actor Object Reference") (OtherComp :type "PrimitiveComponent Object Reference") (OtherBodyIndex :type Integer) (bFromSweep :type Boolean) (SweepResult :type "HitResult Structure (by ref)"))
  (bind _returnvalue (`GameplayStatics.GetPlayerController` 0))
  (bind _asbp_character (cast `/Game/_Main/Blueprints/BP_Character` OtherActor))
  (switch `int` (`self.LevelToLoad`)
    (:`Default`
      (bind _returnvalue_2 (`|CreateWidget` "/Game/_Main/Widget/WBP_WinScreen.WBP_WinScreen_C" _returnvalue :!label _label))
      (`UserWidget.AddToViewport` _returnvalue_2 0))
    (:`0`
      (goto _label))
    (:`2`
      (bind _returnvalue_3 (`|CreateWidget` "/Game/_Main/Widget/WBP_NextLevel.WBP_NextLevel_C" (`GameplayStatics.GetPlayerController` 0)))
      (`UserWidget.AddToViewport` _returnvalue_3 0)))
  (set `PlayerController.bShowMouseCursor` true _returnvalue)
  (`WidgetBlueprintLibrary.SetInputMode_UIOnlyEx` _returnvalue null)
  (set `/Game/_Main/Blueprints/BP_Character.IsGameOver?` true _asbp_character))

(fn `UserConstructionScript`)