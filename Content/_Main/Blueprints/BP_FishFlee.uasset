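; BP_FishFlee is a fish character that flees along a given direction and is removed when the player touches it.
; On BeginPlay it switches its movement component to flying mode.
; The Flee event adds movement input along the normalized direction scaled by Speed.
; An overlap of its sphere with BP_Character prints a debug message and destroys the fish.
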(event `self.ReceiveBeginPlay`
  (set `self.IsDead` false)
  (`CharacterMovementComponent.SetMovementMode` (`self.CharacterMovement`) "MOVE_Flying" 0))

(event `Flee`
  (params (dir :type "Vector Structure"))
  (`self.AddMovementInput` (`KismetMathLibrary.Normal` dir) (`self.Speed`)))

(event `self.Sphere.OnComponentBeginOverlap`
  (params (OverlappedComponent :type "PrimitiveComponent Object Reference") (OtherActor :type "Actor Object Reference") (OtherComp :type "PrimitiveComponent Object Reference") (OtherBodyIndex :type Integer) (bFromSweep :type Boolean) (SweepResult :type "HitResult Structure (by ref)"))
  (cast `/Game/_Main/Blueprints/BP_Character` OtherActor)
  (`KismetSystemLibrary.PrintString` "collided w player" true true (struct :`R` 0.859375 :`G` 0.375278 :`A` 1.0) 3.0)
  (`self.K2_DestroyActor`))

(fn `UserConstructionScript`)