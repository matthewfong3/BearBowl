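; AI controller for BP_FishFlee pawns that makes fish flee when the player comes near.
; It caches the fish on possess, then checks each Tick, while the fish is alive, its distance to player pawn 0.
; Within the fish's FleeRadiusThreshold it calls Flee with the unnormalized away-from-player vector; otherwise it adds zero movement input.
; The logic is pure polling, with no behavior tree or perception.
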(event `self.ReceivePossess`
  (params (PossessedPawn :type "Pawn Object Reference"))
  (bind _asbp_fish_flee (cast `/Game/_Main/Blueprints/BP_FishFlee` PossessedPawn))
  (set `self.BP Fish Flee Ref` _asbp_fish_flee))

(event `self.ReceiveTick`
  (params (DeltaSeconds :type "Float (single-precision)"))
  (bind _bp_fish_flee_ref (`self.BP Fish Flee Ref`))
  (bind _returnvalue (- (`self.K2_GetActorLocation` (`self.BP Fish Flee Ref`)) (`self.K2_GetActorLocation` (`GameplayStatics.GetPlayerPawn` 0))))
  (bind _bp_fish_flee_ref_2 (`self.BP Fish Flee Ref`)
    (:`then`
      (if (not (`/Game/_Main/Blueprints/BP_FishFlee.IsDead` _bp_fish_flee_ref_2))
        (if (<= (`KismetMathLibrary.VSize` (`KismetMathLibrary.Vector_GetAbs` _returnvalue)) (`/Game/_Main/Blueprints/BP_FishFlee.FleeRadiusThreshold` (`self.BP Fish Flee Ref`)))
          (`/Game/_Main/Blueprints/BP_FishFlee.Flee` _bp_fish_flee_ref _returnvalue)
          (else
            (`Pawn.AddMovementInput` _bp_fish_flee_ref (0.0 0.0 0.0) 1.0 false)))))
    (:`else`)))

(fn `UserConstructionScript`)