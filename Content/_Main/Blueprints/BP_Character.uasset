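; Player character for a side-scrolling swimming game, collecting fleeing fish while managing a depleting oxygen supply.
; Enhanced Input drives horizontal movement with left/right facing flips, upward swim launches, and pause toggling on the HUD it creates.
; A looping timer drains oxygen unless paused and opens the lose screen at zero, while ReplenishOxygen restores it.
; Box overlaps count and destroy fish; the flipbook animation logic is never run.
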(event `self.ReceiveBeginPlay`
  (bind _asplayer_controller (cast `PlayerController` (`self.GetController`)))
  (`EnhancedInputSubsystemInterface.AddMappingContext` (pcsubsystem `EnhancedInputLocalPlayerSubsystem` _asplayer_controller) "/Game/_Main/Input/IMC_Default.IMC_Default" 0 (struct))
  (`WidgetBlueprintLibrary.SetInputMode_GameOnly` _asplayer_controller)
  (bind _returnvalue (`|CreateWidget` "/Game/_Main/Widget/WBP_InGame.WBP_InGame_C" (`GameplayStatics.GetPlayerController` 0)))
  (bind _output_get (set `self.WBP_HUD` _returnvalue))
  (`UserWidget.AddToViewport` _output_get 0)
  (bind _returnvalue_2 (`KismetSystemLibrary.K2_SetTimerDelegate` (delegate `DepleteOxygen`) (`self.OxygenTimerTickDuration`) true))
  (set `self.OxygenTimerHandle` _returnvalue_2))

(event `DepleteOxygen`
  (if (> (`self.Oxygen`) 0.0)
    (if (not (`self.IsGamePaused?`))
      (set `self.Oxygen` (- (`self.Oxygen`) (`self.OxygenDepletionRate`))))
    (else
      (`self.Death`)
      (`KismetSystemLibrary.K2_ClearAndInvalidateTimerHandle` (`self.OxygenTimerHandle`)))))

(event `self.ReceiveTick`
  (params (DeltaSeconds :type "Float (single-precision)")))

(event `EnhancedInput|/Game/_Main/Input/Actions/IA_Jump`
  (params (ActionValue :type Boolean) (ElapsedSeconds :type "Float (double-precision)") (TriggeredSeconds :type "Float (double-precision)") (InputAction :type "InputAction Object Reference" :default "/Game/_Main/Input/Actions/IA_Jump.IA_Jump"))
  (:`Started`
    (`self.LaunchCharacter` (`KismetMathLibrary.MakeVector` 0.0 0.0 (`self.VerticalSwimForce`)) false true)))

(event `Death`
  (`GameplayStatics.OpenLevelBySoftObjectPtr` "/Game/_Main/Maps/M_LoseScreen.M_LoseScreen"))

(event `EnhancedInput|/Game/_Main/Input/Actions/IA_Move`
  (params (ActionValue :type "Float (double-precision)") (ElapsedSeconds :type "Float (double-precision)") (TriggeredSeconds :type "Float (double-precision)") (InputAction :type "InputAction Object Reference" :default "/Game/_Main/Input/Actions/IA_Move.IA_Move"))
  (:`Triggered`
    (`self.AddMovementInput` (1.0 0.0 0.0) (* ActionValue (`self.Speed`)))
    (`Controller.SetControlRotation` (`self.GetController`) (select `bool` (> ActionValue 0.0) :`false` (`KismetMathLibrary.MakeRotator` 0.0 0.0 180.0) :`true` (`KismetMathLibrary.MakeRotator` 0.0)))))

(event `EnhancedInput|/Game/_Main/Input/Actions/IA_Pause`
  (params (ActionValue :type Boolean) (ElapsedSeconds :type "Float (double-precision)") (TriggeredSeconds :type "Float (double-precision)") (InputAction :type "InputAction Object Reference" :default "/Game/_Main/Input/Actions/IA_Pause.IA_Pause"))
  (:`Started`
    (`/Engine/EditorBlueprintResources/StandardMacros.FlipFlop`
      (:`A`
        _)
      (:`B`
        _))
    (`/Game/_Main/Widget/WBP_InGame.TogglePauseMenu` (`self.WBP_HUD`))))

(event `self.Box.OnComponentBeginOverlap`
  (params (OverlappedComponent :type "PrimitiveComponent Object Reference") (OtherActor :type "Actor Object Reference") (OtherComp :type "PrimitiveComponent Object Reference") (OtherBodyIndex :type Integer) (bFromSweep :type Boolean) (SweepResult :type "HitResult Structure (by ref)"))
  (bind _asbp_fish_flee (cast `/Game/_Main/Blueprints/BP_FishFlee` OtherActor))
  (`/Engine/EditorBlueprintResources/StandardMacros.IncrementInt` (`self.TotalFishCollected`)
    (:`  `
      (`self.K2_DestroyActor` _asbp_fish_flee))))

(event `ReplenishOxygen`
  (params (OxygenAmount :type "Float (double-precision)"))
  (set `self.Oxygen` (`KismetMathLibrary.FClamp` (+ (`self.Oxygen`) OxygenAmount) 0.0 100.0)))

(fn `UpdateAnimation`
  (bind (_returnvalue_x _returnvalue_y _returnvalue_z) (`KismetMathLibrary.BreakVector` (`self.GetVelocity`)))
  (bind _sprite (`self.Sprite`))
  (bind _sprite_2 (`self.Sprite`))
  (if (`NavMovementInterface.IsMovingOnGround` (`self.CharacterMovement`))
    (if (> (`KismetMathLibrary.VSize` (`self.GetVelocity`)) 0.0)
      ; Set Running Flipbook
      (`PaperFlipbookComponent.SetFlipbook` _sprite_2 null)
      (else
        ; Set Idle Flipbook
        (`PaperFlipbookComponent.SetFlipbook` _sprite_2 null)))
    (elif (< _returnvalue_z -100.0)
      ; Fall
      (`PaperFlipbookComponent.SetFlipbook` _sprite null)
      (else
        ; Jump Rise
        (`PaperFlipbookComponent.SetFlipbook` _sprite null)))))

(fn `UserConstructionScript`)