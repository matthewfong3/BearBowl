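; BP_Swordfish is an enemy that charges when the player character enters its attack zone and damages the player on contact.
; The Attack overlap waits for AttackPause, then applies a large CharacterMovement force along world X, signed by the capsule's relative yaw.
; A separate HurtBox overlap calls OnDamage on BP_Character with the Damage value.
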(event `self.Attack.OnComponentBeginOverlap`
  (params (OverlappedComponent :type "PrimitiveComponent Object Reference") (OtherActor :type "Actor Object Reference") (OtherComp :type "PrimitiveComponent Object Reference") (OtherBodyIndex :type Integer) (bFromSweep :type Boolean) (SweepResult :type "HitResult Structure (by ref)"))
  (bind _charactermovement (`self.CharacterMovement`))
  ; Charge If Player is In Front
  (cast `/Game/_Main/Blueprints/BP_Character` OtherActor)
  (`KismetSystemLibrary.Delay` (`self.AttackPause`))
  (if (> (.yaw (.rotation (`SceneComponent.GetRelativeTransform` (`self.CapsuleComponent`)))) 0.0)
    (`CharacterMovementComponent.AddForce` _charactermovement (10000000.0 0.0 0.0))
    (else
      (`CharacterMovementComponent.AddForce` _charactermovement (-10000000.0 0.0 0.0)))))

(event `self.HurtBox.OnComponentBeginOverlap`
  (params (OverlappedComponent :type "PrimitiveComponent Object Reference") (OtherActor :type "Actor Object Reference") (OtherComp :type "PrimitiveComponent Object Reference") (OtherBodyIndex :type Integer) (bFromSweep :type Boolean) (SweepResult :type "HitResult Structure (by ref)"))
  ; Hurt Player If You Hit
  (bind _asbp_character (cast `/Game/_Main/Blueprints/BP_Character` OtherActor))
  (`/Game/_Main/Interfaces/BPI_Bear.OnDamage` _asbp_character (`self.Damage`)))

(fn `UserConstructionScript`)